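; Grappling hook item that fires a cabled hook and pulls the player toward surfaces of the hookshot material class.
; A camera line trace sets the goal, then timelines fly the spawned hook out, move the player with swept lerps at distance-scaled speed, and retract it.
; Tick, enabled during shots, updates the cable, correcting its start for the on-top material's FOV modifier.
; Item switching stays locked until the hook resets.
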(event `self.ReceiveBeginPlay`
  (`parent.ReceiveBeginPlay`))

(event `self.Secondary Action`)

(event `self.ReceiveTick`
  (params (DeltaSeconds :type "Float (single-precision)"))
  (bind _returnvalue (`GameplayStatics.GetPlayerCameraManager` 0))
  (bind _hook (`self.Hook`))
  (bind _returnvalue_2 (`PlayerCameraManager.GetCameraLocation` _returnvalue))
  (bind _returnvalue_3 (`KismetMathLibrary.GetForwardVector` (`PlayerCameraManager.GetCameraRotation` _returnvalue)))
  (bind _returnvalue_4 (- (`SceneComponent.K2_GetComponentLocation` (`self.CablePlace`)) _returnvalue_2))
  ;[1 1 1] Tick setting the cable
  (`parent.ReceiveTick` DeltaSeconds)
  (if (`KismetSystemLibrary.IsValid` _hook)
    (`SceneComponent.K2_SetWorldLocation` (`self.HookLocation`) (`SceneComponent.K2_GetComponentLocation` (`/Game/Anachronia/Blueprints/ItemsAndWeapons/HookItem.HookBottom` _hook)) false false)
    (set `CableComponent.EndLocation` (`SceneComponent.RelativeLocation` (`self.HookLocation`)) (`self.Cable`))
    (`SceneComponent.K2_SetWorldLocation` (`self.Cable`) (+ (+ (* (- (* _returnvalue_3 (`KismetMathLibrary.Dot_VectorVector` _returnvalue_3 _returnvalue_4)) _returnvalue_4) (- 1.0 (/ (`KismetMathLibrary.DegreesToRadians` (`PlayerCameraManager.GetFOVAngle` _returnvalue)) (`KismetMathLibrary.DegreesToRadians` 90.0)))) _returnvalue_4) _returnvalue_2) false false)))

(event `self.Primary Action`
  ;[1 1 1] 1. Click
  (if (not (`self.IsShooting`))
    (bind _asg_hook_anim_bp (cast `/Game/Anachronia/Blueprints/gHook_Anim_BP` (`SkeletalMeshComponent.GetAnimInstance` (`self.Grappling_Hook`))))
    (set `/Game/Anachronia/Blueprints/gHook_Anim_BP.isShooting` true _asg_hook_anim_bp)
    (set `self.IsShooting` true)
    (bind _asanachronia_player_bp (cast `/Game/FirstPersonCPP/Blueprints/AnachroniaPlayerBP` (`self.AttachedPlayer`))
      (:`then`
        (set `/Game/FirstPersonCPP/Blueprints/AnachroniaPlayerBP.CanSwitchItem` false _asanachronia_player_bp))
      (:`CastFailed`
        _))
    (`self.HookShotTest`)
    (`KismetSystemLibrary.Delay` 0.2)
    (set `/Game/Anachronia/Blueprints/gHook_Anim_BP.isShooting` false _asg_hook_anim_bp)))

(event `HookShotTest`
  (bind _firstpersoncameracomponent (`AnachroniaPlayer.FirstPersonCameraComponent` (`self.AttachedPlayer`)))
  (bind _returnvalue (`SceneComponent.K2_GetComponentLocation` _firstpersoncameracomponent))
  (bind _returnvalue_2 (`KismetMathLibrary.GetForwardVector` (`SceneComponent.K2_GetComponentRotation` _firstpersoncameracomponent)))
  ;[1 1 1] 2. Linetrace
  (bind _outhit (`KismetSystemLibrary.LineTraceSingle` (+ _returnvalue _returnvalue_2) (+ _returnvalue (* _returnvalue_2 2500)) "TraceTypeQuery1"))
  (bind _output_get (set `self.Hit` (`GameplayStatics.BreakHitResult` _outhit)))
  (if _output_get
    (set `self.HitLocation` (`.Location` (`GameplayStatics.BreakHitResult` _outhit)))
    (set `self.HitDistance` (`.Distance` (`GameplayStatics.BreakHitResult` _outhit)))
    (bind _returnvalue_3 (`GameplayStatics.GetObjectClass` (`.HitActor` (`GameplayStatics.BreakHitResult` _outhit))))
    (if (`KismetSystemLibrary.IsValidClass` _returnvalue_3)
      (set `self.HitClass` _returnvalue_3)
      (else
        (set `self.HitClass` "/Game/Anachronia/Blueprints/ItemsAndWeapons/NothingItem.NothingItem_C"))))
  (`self.Shoot Hook`))

(event `Shoot Hook`
  (bind _grapplinghook_hook (`self.Grapplinghook_Hook`))
  (bind _hook (`self.Hook`))
  ;[1 1 1] 3. Shoot Hook
  (`/Engine/EditorBlueprintResources/StandardMacros.IsValid` _hook
    (:`Is Valid`
      (`self.K2_DestroyActor` _hook))
    (:`Is Not Valid`
      _))
  (`SceneComponent.SetVisibility` _grapplinghook_hook false false)
  (bind _returnvalue (`|SpawnActorFromClass` "/Game/Anachronia/Blueprints/ItemsAndWeapons/HookItem.HookItem_C" (`SceneComponent.K2_GetComponentToWorld` _grapplinghook_hook) "Undefined" "OverrideRootScale" null null))
  (set `self.Hook` _returnvalue)
  (`SceneComponent.SetHiddenInGame` (`self.Cable`) false false)
  (`self.SetActorTickEnabled` true)
  (bind _returnvalue_2 (`FMODBlueprintStatics.PlayEvent2D` "/Game/FMOD/Events/Karaktär/Tools/HookShot.HookShot"))
  (set `self.Soundeffect` _returnvalue_2)
  (`FMODBlueprintStatics.EventInstanceSetParameter` _returnvalue_2 "Hit_reg" 1.0)
  (if (`self.Hit`)
    (`FMODBlueprintStatics.EventInstanceSetParameter` (struct) "Miss")
    (else
      (`FMODBlueprintStatics.EventInstanceSetParameter` (struct) "Miss" 1.0)))
  (`self.LocationForHook`))

(event `LocationForHook`
  (bind _firstpersoncameracomponent (`AnachroniaPlayer.FirstPersonCameraComponent` (`self.AttachedPlayer`)))
  (bind _returnvalue (`SceneComponent.K2_GetComponentRotation` _firstpersoncameracomponent))
  (bind _returnvalue_2 (`SceneComponent.K2_GetComponentLocation` _firstpersoncameracomponent))
  (bind _returnvalue_3 (`KismetMathLibrary.GetForwardVector` _returnvalue))
  ;[1 1 1] 4. Location Setter
  (if (`self.Hit`)
    (set `self.Goal` (`KismetMathLibrary.MakeTransform` (+ _returnvalue_2 (* _returnvalue_3 (- (`self.HitDistance`) 10.0))) _returnvalue))
    (else
      (bind _output_get (set `self.Goal` (`KismetMathLibrary.MakeTransform` (+ (* _returnvalue_3 2500) _returnvalue_2) _returnvalue)))))
  (bind _output_get_2 (set `self.Start` (`SceneComponent.K2_GetComponentToWorld` (`self.Grapplinghook_Hook`))))
  (bind (_direction _other _rotation) (`Timeline|HookFlying` :!via `PlayFromStart`)
    (:`Update`
      (`SceneComponent.K2_SetWorldTransform` (`Actor.RootComponent` (`self.Hook`)) (`KismetMathLibrary.MakeTransform` (`KismetMathLibrary.VLerp` (.location _output_get_2) (.location _output_get) _other) (`KismetMathLibrary.RLerp` (.rotation _output_get_2) (.rotation _output_get) _rotation true)) true false))
    (:`Finished`
      (if (`self.Hit`)
        (`self.CanHook`)
        (else
          (`self.Reset Hook`))))))

(event `StopHookshot`
  ;[1 1 1] 5. Move player
  (`self.Reset Hook`)
  (`Character.LaunchCharacter` (`self.AttachedPlayer`) (0.0 0.0 100.0) false true)
  (bind (_direction _hookshot_speed_track) (`Timeline|Hookshot` :!via `Stop` :!label _label)
    (:`Update`
      (bind _sweephitresult (`SceneComponent.K2_SetWorldLocation` (`Actor.RootComponent` (`self.AttachedPlayer`)) (`KismetMathLibrary.VLerp` (stale `CanHook` _output_get) (`self.HitLocation`) _hookshot_speed_track) true false))
      (if (`GameplayStatics.BreakHitResult` _sweephitresult)
        (`self.StopHookshot`)))))

(event `CanHook`
  ;[1 1 1] 5. Move player
  (if (== (`self.HitClass`) "/Game/Anachronia/Blueprints/Others/HookShotMaterial.HookShotMaterial_C")
    (bind _output_get (set `self.LerpHook` (`SceneComponent.K2_GetComponentLocation` (`Character.CapsuleComponent` (`self.AttachedPlayer`)))))
    (`TimelineComponent.SetPlayRate` (`self.Hookshot`) (/ 1.0 (+ (/ (`self.HitDistance`) 1000.0) 0.5)))
    (goto _label :!via `PlayFromStart`)
    (else
      (`self.Reset Hook`))))

(event `Reset Hook`
  (bind _grapplinghook_hook (`self.Grapplinghook_Hook`))
  (bind _hook (`self.Hook`))
  ;[1 1 1] 6. Reset Hook Back to it's position
  (`FMODBlueprintStatics.EventInstanceSetParameter` (`self.Soundeffect`) "Miss" 1.0)
  (bind _output_get (set `self.Start` (`self.GetTransform` _hook)))
  (bind (_direction _newtrack_0) (`Timeline|ResetHookTL` :!via `PlayFromStart`)
    (:`Update`
      (`SceneComponent.K2_SetRelativeTransform` (`Actor.RootComponent` (`self.Hook`)) (`KismetMathLibrary.TLerp` _output_get (`SceneComponent.K2_GetComponentToWorld` _grapplinghook_hook) _newtrack_0) false true))
    (:`Finished`
      (`self.K2_DestroyActor` _hook)
      (`SceneComponent.SetVisibility` _grapplinghook_hook true false)
      (`SceneComponent.SetHiddenInGame` (`self.Cable`) true false)
      (bind _asanachronia_player_bp (cast `/Game/FirstPersonCPP/Blueprints/AnachroniaPlayerBP` (`self.AttachedPlayer`)))
      (set `/Game/FirstPersonCPP/Blueprints/AnachroniaPlayerBP.CanSwitchItem` true _asanachronia_player_bp)
      (`self.SetActorTickEnabled` false)
      (`KismetSystemLibrary.Delay` 0.5)
      (set `self.IsShooting` false))))

(fn `NewFunction_0`
  (params (self2 :type "SceneComponent Object Reference")))

(fn `UserConstructionScript`
  (`parent.UserConstructionScript`))