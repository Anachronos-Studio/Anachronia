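; Shock gun weapon Blueprint that flags itself as a weapon and offers a primary action and a charged secondary action.
; Primary action only spends one ammo.
; Holding secondary runs a looping IncreaseDamage timer that drains two ammo per call and sets output damage to base times multiplier, without accumulating.
; Release clears the timer and prints damage and ammo; no firing or damage application happens here.
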(event `self.ReceiveBeginPlay`
  (`parent.ReceiveBeginPlay`)
  (set `self.bIsWeapon` true)
  (set `self.TagName` (`self.TagName`)))

(event `InputAction|SecondaryAction`
  (params (Key :type "Key Structure"))
  (:`Pressed`
    (bind _returnvalue (`KismetSystemLibrary.K2_SetTimer` null "IncreaseDamage" 0.0 true)) ; Timer for charge
  )
  (:`Released`
    (`KismetSystemLibrary.K2_ClearAndInvalidateTimerHandle` _returnvalue)
    (`KismetSystemLibrary.PrintString` (`KismetStringLibrary.Concat_StrStr` "Output Damage:" (`KismetStringLibrary.Conv_DoubleToString` (`self.OutputDamage`))) true true (struct :`G` 0.525951 :`B` 1.0 :`A` 1.0))
    (`KismetSystemLibrary.PrintString` (`KismetStringLibrary.Concat_StrStr` "Ammo:" (`KismetStringLibrary.Conv_DoubleToString` (`self.WeaponAmmo`))) true true (struct :`R` 0.625 :`A` 1.0))))

(event `self.Primary Action`
  (set `self.WeaponAmmo` (+ (`self.WeaponAmmo`) -1.0)))

(event `self.ReceiveTick`
  (params (DeltaSeconds :type "Float (single-precision)")))

(fn `IncreaseDamage`
  (set `self.WeaponAmmo` (+ (`self.WeaponAmmo`) -2.0))
  (set `self.OutputDamage` (* (`self.BaseWeaponDamage`) (`self.DamageMultiplier`))))

(fn `UserConstructionScript`
  (`parent.UserConstructionScript`))