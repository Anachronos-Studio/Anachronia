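; Cable cutter item Blueprint that lets the player holding it interact with the world.
; Its primary action casts the attached player to AnachroniaPlayerBP and calls InteractFromItem, so the item itself contains no cutting logic.
; The secondary action is empty, the standard BeginPlay, overlap and Tick events are disabled, and NewFunction_0 is an unused stub.
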(event `self.Secondary Action`)

(event `self.Primary Action`
  (bind _asanachronia_player_bp (cast `/Game/FirstPersonCPP/Blueprints/AnachroniaPlayerBP` (`self.AttachedPlayer`)))
  (`/Game/FirstPersonCPP/Blueprints/AnachroniaPlayerBP.Interact From Item` _asanachronia_player_bp))

(fn `NewFunction_0`
  (params (self2 :type "SceneComponent Object Reference")))

(fn `UserConstructionScript`
  (`parent.UserConstructionScript`))