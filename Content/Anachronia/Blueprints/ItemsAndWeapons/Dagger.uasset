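; Dagger is a melee weapon item for the Anachronia player that slashes guards and deals bonus damage on stealth hits.
; The primary action sets a timed slashing flag on the gHook anim blueprint and plays a sword sound.
; Guards overlapping its box during a slash take the player's lethal damage plus base weapon damage, multiplied by a stealth factor unless the guard's AI alertness is Alarmed Knowing.
; Secondary action is an empty stub.
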(event `self.ReceiveBeginPlay`
  (`parent.ReceiveBeginPlay`)
  (set `self.bIsWeapon` true)
  (set `self.TagName` (`self.TagName`)))

(event `self.ReceiveTick`
  (params (DeltaSeconds :type "Float (single-precision)"))
  (`parent.ReceiveTick` DeltaSeconds))

(event `self.Primary Action`
  (if (not (`/Game/Anachronia/Blueprints/gHook_Anim_BP.isSlashing` (stale _asg_hook_anim_bp)))
    (bind _asg_hook_anim_bp (cast `/Game/Anachronia/Blueprints/gHook_Anim_BP` (`SkeletalMeshComponent.GetAnimInstance` (`self.SkeletalMesh`))))
    (set `/Game/Anachronia/Blueprints/gHook_Anim_BP.isSlashing` true _asg_hook_anim_bp)
    (`FMODBlueprintStatics.PlayEvent2D` "/Game/FMOD/Events/Karaktär/Tools/Sword.Sword")
    (`KismetSystemLibrary.Delay` 0.65)
    (set `/Game/Anachronia/Blueprints/gHook_Anim_BP.isSlashing` false _asg_hook_anim_bp)))

(event `self.DealLethalDamage`)

(event `self.Secondary Action`)

(event `self.Box.OnComponentEndOverlap`
  (params (OverlappedComponent :type "PrimitiveComponent Object Reference") (OtherActor :type "Actor Object Reference") (OtherComp :type "PrimitiveComponent Object Reference") (OtherBodyIndex :type Integer)))

(event `self.Box.OnComponentBeginOverlap`
  (params (OverlappedComponent :type "PrimitiveComponent Object Reference") (OtherActor :type "Actor Object Reference") (OtherComp :type "PrimitiveComponent Object Reference") (OtherBodyIndex :type Integer) (bFromSweep :type Boolean) (SweepResult :type "HitResult Structure (by ref)"))
  ;[1 1 1] Comment
  (bind _asg_hook_anim_bp (cast `/Game/Anachronia/Blueprints/gHook_Anim_BP` (`SkeletalMeshComponent.GetAnimInstance` (`self.SkeletalMesh`)))
    (:`then`
      (if (`/Game/Anachronia/Blueprints/gHook_Anim_BP.isSlashing` _asg_hook_anim_bp)
        (bind _asbp_guard (cast `/Game/Anachronia/Blueprints/BP_Guard` OtherActor))
        (bind _returnvalue (`GuardPawn.GetGuardAI` _asbp_guard))
        (`/Engine/EditorBlueprintResources/StandardMacros.IsValid` _returnvalue
          (:`Is Valid`
            (switch `EAlertness` (`GuardAIController.Alertness` _returnvalue)
              (:`Neutral`
                (set `self.TargetIsAlarmed` false :!label _label))
              (:`Distracted`
                (goto _label))
              (:`AlarmedKnowing`
                (set `self.TargetIsAlarmed` true))
              (:`AlarmedUnknowing`
                (goto _label)))
            (bind _asanachronia_player_bp (cast `/Game/FirstPersonCPP/Blueprints/AnachroniaPlayerBP` (`self.AttachedPlayer`))
              (:`then`
                (bind _returnvalue_2 (`AnachroniaPlayer.GetLethalDamage` _asanachronia_player_bp))
                (if (`self.TargetIsAlarmed`)
                  (bind _returnvalue_3 (+ _returnvalue_2 (`self.BaseWeaponDamage`)))
                  (`KismetSystemLibrary.PrintString` (`KismetStringLibrary.Conv_DoubleToString` _returnvalue_3))
                  (`GuardPawn.SetDamageToCurrentHealth` _asbp_guard _returnvalue_3 false)
                  (else
                    (bind _returnvalue_4 (* _returnvalue_3 (`self.StealthDamageMultiplier`)))
                    (`KismetSystemLibrary.PrintString` (`KismetStringLibrary.Conv_DoubleToString` _returnvalue_4))
                    (`GuardPawn.SetDamageToCurrentHealth` _asbp_guard _returnvalue_4 false)))
                (`KismetSystemLibrary.Delay` 0.05)
                (`FMODBlueprintStatics.PlayEvent2D` "/Game/FMOD/Events/Karaktär/Tools/Kling.Kling")
                (`KismetSystemLibrary.Delay` 0.1))
              (:`CastFailed`
                (`KismetSystemLibrary.PrintString` (`KismetStringLibrary.Concat_StrStr` (`KismetSystemLibrary.GetDisplayName` _asanachronia_player_bp) " nullptr")))))
          (:`Is Not Valid`
            (`KismetSystemLibrary.PrintString` "nullptr")))))
    (:`CastFailed`
      (`KismetSystemLibrary.PrintString` "Non-attacking collision"))))

(fn `NewFunction_0`
  (params (self2 :type "SceneComponent Object Reference")))

(fn `UserConstructionScript`
  (`parent.UserConstructionScript`))