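; Grappling hook item that pulls the player toward surfaces of the HookShotMaterial actor class.
; PrimaryAction pulses the shooting animation, then line-traces from the first-person camera, with debug drawing, for a valid target.
; A Timeline lerps the player from capsule location to hit point, its play rate scaled by distance.
; The move sweeps, and a blocking hit stops the Timeline and resets velocity to a slight drop.
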(event `self.Primary Action`
  (bind _asg_hook_anim_bp (cast `/Game/Anachronia/Blueprints/gHook_Anim_BP` (`SkeletalMeshComponent.GetAnimInstance` (`self.Grappling_Hook`))))
  (set `/Game/Anachronia/Blueprints/gHook_Anim_BP.isShooting` true _asg_hook_anim_bp)
  (`KismetSystemLibrary.Delay` 0.2)
  (set `/Game/Anachronia/Blueprints/gHook_Anim_BP.isShooting` false _asg_hook_anim_bp)
  (`self.Hook Shot Test`))

(event `StopHookshot`
  (bind _playerthing (`self.PlayerThing`))
  (set `MovementComponent.Velocity` (0.0 0.0 -2.0) (`Pawn.GetMovementComponent` _playerthing))
  (bind (_direction _hookshot_speed_track) (`Timeline|Hookshot` :!via `Stop` :!label _label)
    (:`Update`
      (bind _sweephitresult (`SceneComponent.K2_SetWorldLocation` (`Actor.RootComponent` _playerthing) (`KismetMathLibrary.VLerp` (stale `Hook Shot Test` _output_get) (`.Location` (`GameplayStatics.BreakHitResult` (stale `Hook Shot Test` _outhit))) _hookshot_speed_track) true false))
      (if (`GameplayStatics.BreakHitResult` _sweephitresult)
        (`self.StopHookshot`)))))

(event `Hook Shot Test`
  (bind _firstpersoncameracomponent (`AnachroniaPlayer.FirstPersonCameraComponent` (`self.PlayerThing`)))
  (bind _returnvalue (`SceneComponent.K2_GetComponentLocation` _firstpersoncameracomponent))
  (bind _returnvalue_2 (`KismetMathLibrary.GetForwardVector` (`SceneComponent.K2_GetComponentRotation` _firstpersoncameracomponent)))
  (bind _outhit (`KismetSystemLibrary.LineTraceSingle` :`Start` (+ _returnvalue (* _returnvalue_2 50)) :`End` (+ _returnvalue (* _returnvalue_2 2500)) :`TraceChannel` "TraceTypeQuery1" :`DrawDebugType` "ForDuration"))
  (if (== (`GameplayStatics.GetObjectClass` (`.HitActor` (`GameplayStatics.BreakHitResult` _outhit))) "/Game/Anachronia/IndividualPlaygrounds/Max/Maps/HookShotMaterial.HookShotMaterial_C")
    (`KismetSystemLibrary.Delay` 0.1)
    (bind _output_get (set `self.LerpHook` (`SceneComponent.K2_GetComponentLocation` (`Character.CapsuleComponent` (`self.PlayerThing`)))))
    (`TimelineComponent.SetPlayRate` (`self.Hookshot`) (/ 1.0 (+ (/ (`.Distance` (`GameplayStatics.BreakHitResult` _outhit)) 1000.0) 0.5)))
    (goto _label :!via `PlayFromStart`)))

(fn `UserConstructionScript`
  (`parent.UserConstructionScript`))