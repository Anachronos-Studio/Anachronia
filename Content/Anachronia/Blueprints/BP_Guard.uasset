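; BP_Guard is the guard character, with a suspicion indicator and a body the player can carry once it is down.
; An InteractableGuardBody child actor, sized to the guard's capsule on respawn, enables collision only on death.
; Pickup attaches the guard to the player without collision or shadow, shrinking a "ScaleInDepth" material parameter; putdown reverses this and corrects rotation.
; Tick pins the suspicion widget above the guard, clamped to screen edges.
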(event `PickupBody`
  (params (Player :type "/Game/FirstPersonCPP/Blueprints/AnachroniaPlayerBP Object Reference"))
  ;[1 1 1] Player carrying bodies
  (set `/Game/FirstPersonCPP/Blueprints/AnachroniaPlayerBP.CarriedBody` self Player)
  (`PrimitiveComponent.SetSimulatePhysics` (`self.CapsuleComponent`) false)
  (`self.K2_AttachToComponent` (`/Game/FirstPersonCPP/Blueprints/AnachroniaPlayerBP.CarryBodyAttachPoint` Player) "None" "SnapToTarget" "SnapToTarget" "SnapToTarget" false)
  (`self.SetActorEnableCollision` false)
  (`MaterialInstanceDynamic.SetScalarParameterValue` (`self.DynamicMaterial`) "ScaleInDepth" 0.05)
  (`PrimitiveComponent.SetCastShadow` (`self.Mesh`) false))

(event `PutdownBody`
  ;[1 1 1] Player carrying bodies
  (`self.K2_DetachFromActor` "KeepWorld" "KeepWorld" "KeepWorld")
  (`self.SetActorEnableCollision` true)
  (set `/Game/FirstPersonCPP/Blueprints/AnachroniaPlayerBP.CarriedBody` null (stale `PickupBody` Player))
  (bind _returnvalue (`self.FindBestDeadRotation`))
  (`self.K2_SetActorRotation` _returnvalue true)
  (`MaterialInstanceDynamic.SetScalarParameterValue` (`self.DynamicMaterial`) "ScaleInDepth" 1.0)
  (`PrimitiveComponent.SetCastShadow` (`self.Mesh`) true))

(event `self.OnRespawn`
  (bind _capsulecomponent (`self.CapsuleComponent`))
  ;[1 1 1] Dying and respawning
  (bind _asinteractable_guard_body (cast `/Game/Anachronia/Blueprints/Interactables/World/InteractableGuardBody` (`ChildActorComponent.ChildActor` (`self.Interactable`))))
  (bind _output_get (set `self.InteractableActor` _asinteractable_guard_body))
  (set `/Game/Anachronia/Blueprints/Interactables/World/InteractableGuardBody.GuardOwner` self _output_get)
  (`self.SetActorEnableCollision` _output_get false)
  (bind _capsule (`/Game/Anachronia/Blueprints/Interactables/World/InteractableGuardBody.Capsule` _output_get))
  (`CapsuleComponent.SetCapsuleRadius` _capsule (`CapsuleComponent.CapsuleRadius` _capsulecomponent) false)
  (`CapsuleComponent.SetCapsuleHalfHeight` _capsule (`CapsuleComponent.CapsuleHalfHeight` _capsulecomponent) true))

(event `self.OnDeath`
  (params (bNonLethalDeath :type Boolean))
  ;[1 1 1] Dying and respawning
  (`parent.OnDeath` bNonLethalDeath)
  (`self.SetActorEnableCollision` (`self.InteractableActor`) true))

(event `self.ReceiveBeginPlay`
  ;[1 1 1] BeginPlay and Tick
  (`parent.ReceiveBeginPlay`)
  (bind _returnvalue (`|CreateWidget` "/Game/Anachronia/Blueprints/UI/HUD/SusWidget.SusWidget_C" (`GameplayStatics.GetPlayerController` 0)))
  (set `/Game/Anachronia/Blueprints/UI/HUD/SusWidget.Guard` self _returnvalue)
  (`UserWidget.AddToViewport` _returnvalue 0)
  (bind _returnvalue_2 (`KismetMaterialLibrary.CreateDynamicMaterialInstance` "/Game/Anachronia/Materials/Guard/Guard.Guard"))
  (bind _output_get (set `self.DynamicMaterial` _returnvalue_2))
  (`MaterialInstanceDynamic.SetScalarParameterValue` _output_get "ScaleInDepth" 1.0)
  (`PrimitiveComponent.SetMaterial` (`self.Mesh`) 0 _output_get))

(event `self.ReceiveTick`
  (params (DeltaSeconds :type "Float (single-precision)"))
  ;[1 1 1] BeginPlay and Tick
  (`parent.ReceiveTick` DeltaSeconds)
  (`UserWidget.SetPositionInViewport` (stale `self.ReceiveBeginPlay` _returnvalue) (`HudUtility.FindScreenEdgeLocationForWorldLocation` (+ (`self.K2_GetActorLocation`) (0.0 0.0 110.0)) (30.0 30.0)) true))

(fn `UserConstructionScript`)