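; Cinematic camera actor that takes over the player's view and travels the length of a referenced spline when Show is called.
; A half-speed timeline drives the camera's position along the spline, using the spline's local pitch and yaw with yaw flipped 180 degrees.
; On completion it calls SplineDone on the Anachronia player character and briefly blends the view back to them.
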(event `Show`
  (bind _spline (`/Game/Anachronia/Blueprints/Others/SplineForCamera.Spline` (`self.Spline`)))
  (`PlayerController.SetViewTargetWithBlend` (`GameplayStatics.GetPlayerController` 0) self 0.0 "VTBlend_Linear" 0.0 false)
  (`TimelineComponent.SetPlayRate` (`self.FollowSpline`) 0.5)
  (bind (_direction _newtrack_0) (`Timeline|FollowSpline` :!via `PlayFromStart`)
    (:`Update`
      (bind _returnvalue (`KismetMathLibrary.Lerp` 0.0 (`SplineComponent.GetSplineLength` _spline) _newtrack_0))
      (`SceneComponent.K2_SetWorldTransform` (`self.CameraComponent`) (`KismetMathLibrary.MakeTransform` (`SplineComponent.GetLocationAtDistanceAlongSpline` _spline _returnvalue "World") (`KismetMathLibrary.MakeRotator` 0.0 (.pitch (`SplineComponent.GetRotationAtDistanceAlongSpline` _spline _returnvalue "Local")) (+ (.yaw (`SplineComponent.GetRotationAtDistanceAlongSpline` _spline _returnvalue "Local")) 180.0))) false false))
    (:`Finished`
      (bind _asanachronia_player_bp (cast `/Game/FirstPersonCPP/Blueprints/AnachroniaPlayerBP` (`GameplayStatics.GetPlayerCharacter` 0)))
      (`/Game/FirstPersonCPP/Blueprints/AnachroniaPlayerBP.SplineDone` _asanachronia_player_bp)
      (`PlayerController.SetViewTargetWithBlend` (`GameplayStatics.GetPlayerController` 0) _asanachronia_player_bp 0.2 "VTBlend_Linear" 0.0 false))))

(event `self.ReceiveTick`
  (params (DeltaSeconds :type "Float (single-precision)")))

(fn `UserConstructionScript`)