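; Guard2 is a guard actor that links itself to a suspicion meter widget.
; On BeginPlay it runs the parent logic, casts the SusMeter component's widget to SusWidget and sets itself as that widget's Guard.
; An unwired chain, which never runs, would spawn a Voice line for the player and hold IsTalking for the summed dialogue times to prevent overlapping speech.
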(event `self.ReceiveBeginPlay`
  (`parent.ReceiveBeginPlay`)
  (bind _assus_widget (cast `/Game/Anachronia/Blueprints/UI/HUD/SusWidget` (`WidgetComponent.GetUserWidgetObject` (`self.Sus Meter`))))
  (set `/Game/Anachronia/Blueprints/UI/HUD/SusWidget.Guard` self _assus_widget))

(fn `UserConstructionScript`
  (`parent.UserConstructionScript`))