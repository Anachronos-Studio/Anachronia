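; TutorialGuard is a guard for the tutorial that resets the player when its suspicion is full.
; On BeginPlay it creates a SusWidget linked to itself, then each tick pins it above its head, using a screen-edge location with a margin.
; Tick also polls the guard AI's SusValue and, at exactly 1.0, calls ResetPlayer on every RespawnerTutorial.
; A following loop over all TutorialGuards does nothing.
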(event `self.ReceiveBeginPlay`
  (`parent.ReceiveBeginPlay`)
  (bind _returnvalue (`|CreateWidget` "/Game/Anachronia/Blueprints/UI/HUD/SusWidget.SusWidget_C" (`GameplayStatics.GetPlayerController` 0)))
  (set `/Game/Anachronia/Blueprints/UI/HUD/SusWidget.Guard` self _returnvalue)
  (`UserWidget.AddToViewport` _returnvalue 0))

(event `self.ReceiveTick`
  (params (DeltaSeconds :type "Float (single-precision)"))
  (`parent.ReceiveTick` DeltaSeconds)
  (`UserWidget.SetPositionInViewport` (stale `self.ReceiveBeginPlay` _returnvalue) (`HudUtility.FindScreenEdgeLocationForWorldLocation` (+ (`self.K2_GetActorLocation`) (0.0 0.0 125.0)) (30.0 30.0)) true)
  (if (== (`GuardAIController.SusValue` (`self.GetGuardAI`)) 1.0)
    (bind _outactors (`GameplayStatics.GetAllActorsOfClass` "/Game/Anachronia/Blueprints/Others/RespawnerTutorial.RespawnerTutorial_C"))
    (for _array_element _outactors
      (`/Game/Anachronia/Blueprints/Others/RespawnerTutorial.Reset Player` _array_element))
    (bind _outactors_2 (`GameplayStatics.GetAllActorsOfClass` "TutorialGuard_C"))
    (for _ _outactors_2
      _)))

(fn `UserConstructionScript`
  (`parent.UserConstructionScript`))