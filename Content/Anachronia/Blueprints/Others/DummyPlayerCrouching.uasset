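; Stand-in actor for the crouching player that reports whether its capsule is blocked at its location.
; Each Tick resets the Overlapping flag, then sets it if any overlapping component passes the filter.
; The filter ignores overlapper, player and Door actors, plus any box component.
; BeginPlay runs the same check after a brief delay without the reset, then enables Tick.
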(event `self.ReceiveTick`
  (params (DeltaSeconds :type "Float (single-precision)"))
  (set `self.Overlapping` false)
  (for _array_element (`PrimitiveComponent.GetOverlappingComponents` (`self.Capsule`)) :!label _label
    (bind _returnvalue (`ActorComponent.GetOwner` _array_element))
    (cast `/Game/Anachronia/Blueprints/Others/overlapping/overlapper` _returnvalue
      (:`CastFailed`
        (cast `/Game/FirstPersonCPP/Blueprints/AnachroniaPlayerBP` _returnvalue
          (:`CastFailed`
            (cast `/Game/Anachronia/Blueprints/Interactables/World/Door` _returnvalue
              (:`CastFailed`
                (cast `BoxComponent` _array_element
                  (:`CastFailed`
                    (set `self.Overlapping` true))))))))))
  (`self.SetActorTickEnabled` true))

(event `self.ReceiveBeginPlay`
  (`KismetSystemLibrary.Delay` 0.01)
  (goto _label))

(fn `UserConstructionScript`)