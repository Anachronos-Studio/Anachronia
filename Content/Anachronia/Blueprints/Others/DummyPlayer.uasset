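; DummyPlayer is a stand-in actor that detects whether its capsule overlaps anything other than the player or overlapper actors.
; Each tick it clears the Overlapping flag, then sets it if any actor in the capsule fails both casts to overlapper and AnachroniaPlayerBP.
; BeginPlay runs the same scan after a very short delay, skipping the reset, and then enables ticking.
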(event `self.ReceiveTick`
  (params (DeltaSeconds :type "Float (single-precision)"))
  (set `self.Overlapping` false)
  (bind _output_get (set `self.OverlappingItems` (`PrimitiveComponent.GetOverlappingActors` (`self.Capsule`) null) :!label _label))
  (for _array_element _output_get
    (cast `/Game/Anachronia/Blueprints/Others/overlapping/overlapper` _array_element
      (:`CastFailed`
        (cast `/Game/FirstPersonCPP/Blueprints/AnachroniaPlayerBP` _array_element
          (:`CastFailed`
            (set `self.Overlapping` true))))))
  (`self.SetActorTickEnabled` true))

(event `self.ReceiveBeginPlay`
  (`KismetSystemLibrary.Delay` 0.01)
  (goto _label))

(fn `UserConstructionScript`)