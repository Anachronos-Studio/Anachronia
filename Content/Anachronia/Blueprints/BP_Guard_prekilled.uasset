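; A guard variant that starts the level already dead, serving as a pre-placed body.
; Shortly after the parent BeginPlay runs, it applies massive lethal damage to itself.
; Its death event sets the animator's knocked-out flag, enables collision on the interactable actor and runs a luminance check.
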(event `self.ReceiveBeginPlay`
  (`parent.ReceiveBeginPlay`)
  (`KismetSystemLibrary.Delay` 0.2)
  (`self.SetDamageToCurrentHealth` 9999.0))

(event `self.OnDeath`
  (params (bNonLethalDeath :type Boolean))
  (set `/Game/Anachronia/Blueprints/Guard_Anim_BP.isKnockedOut` true (`self.Animator`))
  (`self.SetActorEnableCollision` (`self.InteractableActor`) true)
  (`self.CheckLuminance`))

(fn `UserConstructionScript`
  (`parent.UserConstructionScript`))