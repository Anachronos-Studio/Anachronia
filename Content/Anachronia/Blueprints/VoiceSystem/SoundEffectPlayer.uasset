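; SoundEffectPlayer is a trigger actor that plays a voice line when the Anachronia player overlaps its box.
; It spawns the configured Voice class at its own transform and sets itself as the VoiceLine's AttachedActor.
; An IsTalking flag blocks re-triggering until a delay equal to the sum of the line's DialogueTime entries ends, so later overlaps can play it again.
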(event `self.Box.OnComponentBeginOverlap`
  (params (OverlappedComponent :type "PrimitiveComponent Object Reference") (OtherActor :type "Actor Object Reference") (OtherComp :type "PrimitiveComponent Object Reference") (OtherBodyIndex :type Integer) (bFromSweep :type Boolean) (SweepResult :type "HitResult Structure (by ref)"))
  (cast `/Game/FirstPersonCPP/Blueprints/AnachroniaPlayerBP` OtherActor)
  (if (not (`self.IsTalking`))
    (set `self.IsTalking` true)
    (bind _returnvalue (`|SpawnActorFromClass` (`self.Voice`) (`self.GetTransform`) "Undefined" "OverrideRootScale" self null))
    (bind _asvoice_line (cast `/Game/Anachronia/Blueprints/VoiceSystem/VoiceLine` _returnvalue))
    (set `/Game/Anachronia/Blueprints/VoiceSystem/VoiceLine.AttachedActor` self _asvoice_line)
    (set `self.StopTalkingTimer` 0.0)
    (for _array_element (`/Game/Anachronia/Blueprints/VoiceSystem/VoiceLine.DialogueTime` _asvoice_line)
      (bind _output_get (set `self.StopTalkingTimer` (+ _array_element (stale _output_get)))))
    (`KismetSystemLibrary.Delay` _output_get)
    (set `self.IsTalking` false)))

(fn `UserConstructionScript`)