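; VoiceLine is a short-lived actor that hands a spoken line and its dialogue text to the player character.
; On BeginPlay it waits briefly, casts the player to AnachroniaPlayerBP and sums the dialogue timings into a total duration.
; It passes the sound, text, timings, priority, location and attached actor to the player's VoiceLineController, then destroys itself after another brief delay.
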(event `self.ReceiveBeginPlay`
  (`KismetSystemLibrary.Delay` 0.01)
  (bind _asanachronia_player_bp (cast `/Game/FirstPersonCPP/Blueprints/AnachroniaPlayerBP` (`GameplayStatics.GetPlayerCharacter` 0)))
  (for _array_element (`self.DialogueTime`)
    (set `self.Time` (+ (`self.Time`) _array_element)))
  (`/Game/FirstPersonCPP/Blueprints/AnachroniaPlayerBP.VoiceLineController` _asanachronia_player_bp (`self.Priority`) (`self.K2_GetActorLocation`) (`self.VoiceLine`) (`self.DialogueText`) (`self.DialogueTime`) (`self.Time`) (`self.AttachedActor`))
  (`KismetSystemLibrary.Delay` 0.01)
  (`self.K2_DestroyActor`))

(fn `UserConstructionScript`)