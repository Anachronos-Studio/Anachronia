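; Base class for readable books that open in a full UI when the player interacts with them.
; Interacting pauses the game, shows the cursor and creates a ReadableUI widget displaying the book's texture with UI-only input.
; It records the book as read under its hover text name.
; It matches that text against class defaults in the AllReadables list, using the index to complete the corresponding "Books" achievement sub-goal.
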(event `self.Interacted`
  (params (Player :type "/Game/FirstPersonCPP/Blueprints/AnachroniaPlayerBP Object Reference") (Component :type "ActorComponent Object Reference"))
  (bind _returnvalue (`GameplayStatics.GetPlayerControllerFromID` 0))
  (`GameplayStatics.SetGamePaused` true)
  (set `PlayerController.bShowMouseCursor` true _returnvalue)
  (bind _returnvalue_2 (`|CreateWidget` "/Game/Anachronia/Blueprints/UI/ReadableUI.ReadableUI_C" _returnvalue "/Game/Anachronia/Blueprints/Readables/Images/Books/Book1.Book1" false null))
  (set `/Game/Anachronia/Blueprints/UI/ReadableUI.bookTexture` (`self.TheBook`) _returnvalue_2)
  (`/Game/Anachronia/Blueprints/UI/ReadableUI.UpdateBook` _returnvalue_2)
  (`UserWidget.AddToViewport` _returnvalue_2 0)
  (`WidgetBlueprintLibrary.SetInputMode_UIOnlyEx` _returnvalue _returnvalue_2)
  (`AnachroniaSaveGame.AddReadBooks` (`KismetStringLibrary.Conv_StringToName` (`self.Hover Over Info`)))
  (bind _returnvalue_3 (`GameplayStatics.CreateSaveGameObject` "/Game/Anachronia/Blueprints/Readables/AllReadables.AllReadables_C"))
  (for (_array_element _array_index) (`/Game/Anachronia/Blueprints/Readables/AllReadables.Readables` _returnvalue_3)
    (if (`KismetStringLibrary.EqualEqual_StrStr` (defaults `Object` _array_element) (`self.Hover Over Info`))
      (`AnachroniaSaveGame.AchieveSubGoal` "Books" _array_index))))

(fn `UserConstructionScript`
  (`parent.UserConstructionScript`))