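; BP_Guard_Patrik is a guard actor in Patrik's playground that hooks itself up to a suspicion meter widget.
; On BeginPlay it runs the parent logic, then casts the SusMeter component's user widget to PatrikSusWidget and sets itself as that widget's GuardPatrik reference.
; The construction script only calls its parent, and the Tick and overlap events are disabled.
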(event `self.ReceiveBeginPlay`
  (`parent.ReceiveBeginPlay`)
  (bind _aspatrik_sus_widget (cast `/Game/Anachronia/IndividualPlaygrounds/Patrik/MapsAndPlayer/PatrikSusWidget` (`WidgetComponent.GetUserWidgetObject` (`self.SusMeter`))))
  (set `/Game/Anachronia/IndividualPlaygrounds/Patrik/MapsAndPlayer/PatrikSusWidget.GuardPatrik` self _aspatrik_sus_widget))

(fn `UserConstructionScript`
  (`parent.UserConstructionScript`))