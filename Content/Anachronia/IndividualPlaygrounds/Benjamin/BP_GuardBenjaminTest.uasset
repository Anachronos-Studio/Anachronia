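; Test guard Blueprint that checks whether suspicion-level changes on the guard reach Blueprint events.
; It prints debug messages when suspicion rises to Inspect or Busted, and when it drops from Busted to Not Sus after losing the player.
; It also prints the name of any overlapping actor and enables input from the first player controller on BeginPlay.
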(event `self.ReceiveActorBeginOverlap`
  (params (OtherActor :type "Actor Object Reference"))
  (`KismetSystemLibrary.PrintString` (`KismetSystemLibrary.GetObjectName` OtherActor)))

(event `self.OnSusLevelIncreased`
  (params (NewSusLevel :type "ESusLevel Enum" :default "NotSus") (OldSusLevel :type "ESusLevel Enum" :default "NotSus"))
  (switch `ESusLevel` NewSusLevel
    (:`Inspect`
      (`KismetSystemLibrary.PrintString` "Blueprint knows guard saw something highly suspicious!"))
    (:`Busted`
      (`KismetSystemLibrary.PrintString` "Blueprint knows that guard saw player!"))))

(event `self.OnSusLevelDecreased`
  (params (NewSusLevel :type "ESusLevel Enum" :default "NotSus") (OldSusLevel :type "ESusLevel Enum" :default "NotSus"))
  (switch `ESusLevel` NewSusLevel
    (:`NotSus`
      (if (`|EnumEquality` OldSusLevel "Busted")
        (`KismetSystemLibrary.PrintString` "Blueprint knows guard lost player after hunting her!")))))

(event `self.ReceiveBeginPlay`
  (`parent.ReceiveBeginPlay`)
  (`self.EnableInput` (`GameplayStatics.GetPlayerController` 0)))

(event `self.ReceiveTick`
  (params (DeltaSeconds :type "Float (single-precision)"))
  (`parent.ReceiveTick` DeltaSeconds))

(fn `UserConstructionScript`
  (`parent.UserConstructionScript`))