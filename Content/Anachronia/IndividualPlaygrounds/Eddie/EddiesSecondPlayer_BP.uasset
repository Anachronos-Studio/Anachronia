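; Eddie's playground player Blueprint, with keyboard shortcuts for exercising the save and achievement systems.
; R and T call save and load, and Y activates the SacrumImperium achievement.
; H prints every entry in the achievements map, reading name, description and achieved state from each class's defaults.
; Unconnected equippable-item nodes never run, and the BeginPlay, overlap and Tick events are disabled.
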(event `InputAction|PrimaryAction`
  (params (Key :type "Key Structure")))

(event `Key|R`
  (params (Key :type "Key Structure"))
  (:`Pressed`
    (`self.SaveGame`)))

(event `Key|T`
  (params (Key :type "Key Structure"))
  (:`Pressed`
    (`self.LoadGame`)))

(event `Key|H`
  (params (Key :type "Key Structure"))
  (:`Pressed`
    (bind _values (`BlueprintMapLibrary.Map_Values` (`self.PlayerAchievementsMap`)))
    (for _array_element _values
      (bind (_name _description _bisachieved) (defaults `Object` _array_element))
      (`KismetSystemLibrary.PrintString` (`KismetStringLibrary.Concat_StrStr` (`KismetStringLibrary.Conv_NameToString` _name) ": " _description "! is achieved: " (`KismetStringLibrary.Conv_BoolToString` _bisachieved)) true true (struct :`G` 0.66 :`B` 1.0 :`A` 1.0) 5.0))))

(event `Key|Y`
  (params (Key :type "Key Structure"))
  (:`Pressed`
    (`self.ActivateAchievement` "SacrumImperium")))

(fn `UserConstructionScript`
  (`parent.UserConstructionScript`))